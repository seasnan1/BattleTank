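; Tank Blueprint with a player-controlled orbit camera for aiming.
; BeginPlay passes the barrel and turret components to the tank through setter calls, and the construction script assigns their meshes.
; AimAzimuth yaws an azimuth gimbal and AimElevation pitches the spring arm, both scaled by delta time, keeping the two camera rotation axes on separate components.
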(event EventBeginPlay
  (Class|Tank|SetBarrelReference (Variables|Default|GetTankBarrel))
  (Class|Tank|SetTurretReference (Variables|Default|GetTurret)))

(event Input|AxisEvents|InputAxisAimAzimuth
  (params (AxisValue :type Float%20%28single-precision%29))
  ;[1 1 1] Camera input binding
  (Transformation|AddLocalRotation (Variables|Default|GetAzimuth%20Gimbal) (Math|Rotator|MakeRotator 0.0 0.0 (* AxisValue (Utilities|Time|GetWorldDeltaSeconds) 1e+02)) false false))

(event Input|AxisEvents|InputAxisAimElevation
  (params (AxisValue :type Float%20%28single-precision%29))
  ;[1 1 1] Camera input binding
  (Transformation|AddLocalRotation (Variables|Default|GetSpringArm) (Math|Rotator|MakeRotator 0.0 (* AxisValue (Utilities|Time|GetWorldDeltaSeconds) 1e+01) 0.0) false false))

(fn ConstructionScript
  (Components|StaticMesh|SetStaticMesh (Variables|Default|GetTankBarrel) "/Game/Tank/tank_fbx_Barrel.tank_fbx_Barrel")
  (Components|StaticMesh|SetStaticMesh (Variables|Default|GetTurret) "/Game/Tank/tank_fbx_Turret.tank_fbx_Turret"))